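; Behavior tree task that sends an AI-controlled pawn to the capture point actor stored in the PointToCapture blackboard key.
; On execute it casts the owner to BaseAIController_BP, caches that reference, and runs AI MoveTo on the controlled pawn.
; The task finishes only when the move succeeds, reporting failure even then; a failed move or cast never finishes it.
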(event EventReceiveExecute
  (params (OwnerActor :type Actor%20Object%20Reference))
  (if (!= (Variables|Default|GetAI_Con_Ref) 0)
    _
    (else
      (bind _asbase_aicontroller_bp (Utilities|Casting|CastToBaseAIController_BP OwnerActor))
      (Variables|Default|SetAI_Con_Ref _asbase_aicontroller_bp)))
  (AI|AIMoveTo (Pawn|GetControlledPawn (Variables|Default|GetAI_Con_Ref)) "0, 0, 0" (AI|BehaviorTree|GetBlackboardValueasActor (Variables|Default|GetPointToCapture)) 5.0 false
    (:OnSuccess
      (AI|BehaviorTree|FinishExecute false))))